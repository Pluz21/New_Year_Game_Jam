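; BP_LockTumbler is a lock tumbler that spins its mesh forward or backward on the roll axis, triggered here by the 9 and 0 keys.
; Each direction plays a timeline behind a DoOnce gate, then updates the stored rotation, which wraps to zero at its limit.
; NumberCheck derives TumblerNumber from that rotation after each spin.
; BeginPlay can optionally pick a starting rotation from RandomRotations.
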(event `Key|Zero`
  (params (Key :type "Key Structure"))
  (:`Pressed`
    (`self.SpinTumblerBackward`)))

(event `Key|Nine`
  (params (Key :type "Key Structure"))
  (:`Pressed`
    (`self.SpinTumbler`)))

(event `self.ReceiveBeginPlay`
  (if (`self.randomizeRotation`)
    (`self.RandomizeTumblerRotation`)))

(event `SpinTumbler`
  ;[1 1 1] Spinning
  (`/Engine/EditorBlueprintResources/StandardMacros.DoOnce` false :!label _label
    (:`Completed`
      (bind (_direction _alpha) (`Timeline|timeline` :!via `PlayFromStart`)
        (:`Update`
          (bind _returnvalue (+ (`self.tumblerRotation`) _alpha))
          (`SceneComponent.K2_SetRelativeRotation` (`self.TumblerMesh`) (`KismetMathLibrary.MakeRotator` _returnvalue) false false))
        (:`Finished`
          (set `self.tumblerRotation` _returnvalue)
          (`self.NumberCheck`)
          (`self.SpinTumblerReset`)
          (if (>= (`self.tumblerRotation`) (`self.maxRotation`))
            (set `self.tumblerRotation` 0.0)))))))

(event `SpinTumblerReset`
  ;[1 1 1] Spinning
  (goto _label :!via `Reset`))

(event `SpinTumblerBackward`
  ;[1 1 1] BackwardSpinning
  (`/Engine/EditorBlueprintResources/StandardMacros.DoOnce` false :!label _label_2
    (:`Completed`
      (bind (_direction _alpha) (`Timeline|Timeline_0` :!via `PlayFromStart`)
        (:`Update`
          (bind _returnvalue (- (`self.tumblerRotation`) _alpha))
          (`SceneComponent.K2_SetRelativeRotation` (`self.TumblerMesh`) (`KismetMathLibrary.MakeRotator` _returnvalue) false false))
        (:`Finished`
          (set `self.tumblerRotation` _returnvalue)
          (`self.NumberCheck`)
          (`self.SpinTumblerBackwardReset`)
          (if (<= (`self.tumblerRotation`) (`self.minRotation`))
            (set `self.tumblerRotation` 0.0)))))))

(event `SpinTumblerBackwardReset`
  ;[1 1 1] BackwardSpinning
  (goto _label_2 :!via `Reset`))

(fn `NumberCheck`
  (for _index (range (+ (`self.totalTumblerNumbers`) 1))
    (bind _returnvalue (* _index (`KismetMathLibrary.FTrunc` (`self.tumblerRotation`))))
    (if (== (/ _returnvalue (`self.totalTumblerNumbers`)) _index)
      (if (== _returnvalue 360)
        (set `self.tumblerNumber` _index)
        (else
          (set `self.tumblerNumber` 0)
          (for _index_2 (range (+ (`self.totalTumblerNumbers`) 1))
            (bind _returnvalue_2 (* _index_2 (`KismetMathLibrary.FTrunc` (* (`self.tumblerRotation`) -1.0))))
            (if (== (/ _returnvalue_2 (`self.totalTumblerNumbers`)) _index_2)
              (if (== _returnvalue_2 360)
                (set `self.tumblerNumber` _index_2)
                (else
                  (set `self.tumblerNumber` 0))))))))))

(fn `RandomizeTumblerRotation`
  (bind _randomrotations (`self.randomRotations`))
  (bind _output_get (set `self.tumblerRotation` (`|GetArrayItem` _randomrotations (`KismetMathLibrary.RandomIntegerInRange` (- (`KismetArrayLibrary.Array_Length` _randomrotations) 1)))))
  (`SceneComponent.K2_SetRelativeRotation` (`self.TumblerMesh`) (`KismetMathLibrary.MakeRotator` _output_get) false false)
  (`self.NumberCheck`))

(fn `UserConstructionScript`)