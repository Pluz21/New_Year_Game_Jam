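; Test Blueprint for one lock tumbler that spins forward on key 9 and backward on key 0, optionally starting at a random preset rotation.
; DoOnce-gated Timelines animate the mesh's roll, then update TumblerRotation, which resets to zero at its limits.
; NumberCheck maps 36-degree steps to TumblerNumber through a hardcoded branch chain, storing degree values rather than digits, with negative angles mapped differently.
; Its loop-based calculation is left disconnected.
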(event `Key|Zero`
  (params (Key :type "Key Structure"))
  (:`Pressed`
    (`self.SpinTumblerBackward`)))

(event `Key|Nine`
  (params (Key :type "Key Structure"))
  (:`Pressed`
    (`self.SpinTumbler`)))

(event `self.ReceiveBeginPlay`
  (if (`self.randomizeRotation`)
    (`self.RandomizeTumblerRotation`)))

(event `SpinTumbler`
  ;[1 1 1] Spinning
  (`/Engine/EditorBlueprintResources/StandardMacros.DoOnce` false :!label _label
    (:`Completed`
      (bind (_direction _alpha) (`Timeline|timeline` :!via `PlayFromStart`)
        (:`Update`
          (bind _returnvalue (+ (`self.tumblerRotation`) _alpha))
          (`SceneComponent.K2_SetRelativeRotation` (`self.TumblerMesh`) (`KismetMathLibrary.MakeRotator` _returnvalue) false false))
        (:`Finished`
          (set `self.tumblerRotation` _returnvalue)
          (`self.NumberCheck`)
          (`self.SpinTumblerReset`)
          (if (>= (`self.tumblerRotation`) (`self.maxRotation`))
            (set `self.tumblerRotation` 0.0)))))))

(event `SpinTumblerReset`
  ;[1 1 1] Spinning
  (goto _label :!via `Reset`))

(event `SpinTumblerBackward`
  ;[1 1 1] BackwardSpinning
  (`/Engine/EditorBlueprintResources/StandardMacros.DoOnce` false :!label _label_2
    (:`Completed`
      (bind (_direction _alpha) (`Timeline|Timeline_0` :!via `PlayFromStart`)
        (:`Update`
          (bind _returnvalue (- (`self.tumblerRotation`) _alpha))
          (`SceneComponent.K2_SetRelativeRotation` (`self.TumblerMesh`) (`KismetMathLibrary.MakeRotator` _returnvalue) false false))
        (:`Finished`
          (set `self.tumblerRotation` _returnvalue)
          (`self.NumberCheck`)
          (`self.SpinTumblerBackwardReset`)
          (if (<= (`self.tumblerRotation`) (`self.minRotation`))
            (set `self.tumblerRotation` 0.0)))))))

(event `SpinTumblerBackwardReset`
  ;[1 1 1] BackwardSpinning
  (goto _label_2 :!via `Reset`))

(fn `GetTumblerNumber`
  (returns (tumblerNumber :type Integer))
  (return (`self.tumblerNumber`)))

(fn `LoopBodyNumberCheck`
  (if (== (`KismetMathLibrary.FTrunc` (`self.tumblerRotation`)) 0)
    (set `self.tumblerNumber` 0)
    (elif (== (`KismetMathLibrary.FTrunc` (`self.tumblerRotation`)) 36)
      (set `self.tumblerNumber` 36)
      (elif (== (`KismetMathLibrary.FTrunc` (`self.tumblerRotation`)) 72)
        (set `self.tumblerNumber` 72)
        (elif (== (`KismetMathLibrary.FTrunc` (`self.tumblerRotation`)) 108)
          (set `self.tumblerNumber` 108)
          (elif (== (`KismetMathLibrary.FTrunc` (`self.tumblerRotation`)) 144)
            (set `self.tumblerNumber` 144)
            (elif (== (`KismetMathLibrary.FTrunc` (`self.tumblerRotation`)) 180)
              (set `self.tumblerNumber` 180)
              (elif (== (`KismetMathLibrary.FTrunc` (`self.tumblerRotation`)) 216)
                (set `self.tumblerNumber` 216)
                (elif (== (`KismetMathLibrary.FTrunc` (`self.tumblerRotation`)) 252)
                  (set `self.tumblerNumber` 252)
                  (elif (== (`KismetMathLibrary.FTrunc` (`self.tumblerRotation`)) 288)
                    (set `self.tumblerNumber` 288)
                    (elif (== (`KismetMathLibrary.FTrunc` (`self.tumblerRotation`)) 324)
                      (set `self.tumblerNumber` 324)
                      (elif (== (`KismetMathLibrary.FTrunc` (`self.tumblerRotation`)) 360)
                        (set `self.tumblerNumber` 0)
                        (elif (== (`KismetMathLibrary.FTrunc` (`self.tumblerRotation`)) -36)
                          (set `self.tumblerNumber` 0)
                          (elif (== (`KismetMathLibrary.FTrunc` (`self.tumblerRotation`)) -72)
                            (set `self.tumblerNumber` 36)
                            (elif (== (`KismetMathLibrary.FTrunc` (`self.tumblerRotation`)) -108)
                              (set `self.tumblerNumber` 72)
                              (elif (== (`KismetMathLibrary.FTrunc` (`self.tumblerRotation`)) -144)
                                (set `self.tumblerNumber` 108)
                                (elif (== (`KismetMathLibrary.FTrunc` (`self.tumblerRotation`)) -180)
                                  (set `self.tumblerNumber` 144)
                                  (elif (== (`KismetMathLibrary.FTrunc` (`self.tumblerRotation`)) -216)
                                    (set `self.tumblerNumber` 180)
                                    (elif (== (`KismetMathLibrary.FTrunc` (`self.tumblerRotation`)) -252)
                                      (set `self.tumblerNumber` 216)
                                      (elif (== (`KismetMathLibrary.FTrunc` (`self.tumblerRotation`)) -288)
                                        (set `self.tumblerNumber` 252)
                                        (elif (== (`KismetMathLibrary.FTrunc` (`self.tumblerRotation`)) -324)
                                          (set `self.tumblerNumber` 288)
                                          (elif (== (`KismetMathLibrary.FTrunc` (`self.tumblerRotation`)) -360)
                                            (set `self.tumblerNumber` 0)))))))))))))))))))))))

(fn `NumberCheck`
  (`self.LoopBodyNumberCheck`))

(fn `RandomizeTumblerRotation`
  (bind _randomrotations (`self.randomRotations`))
  (bind _output_get (set `self.tumblerRotation` (`|GetArrayItem` _randomrotations (`KismetMathLibrary.RandomIntegerInRange` 0 (- (`KismetArrayLibrary.Array_Length` _randomrotations) 1)))))
  (`SceneComponent.K2_SetRelativeRotation` (`self.TumblerMesh`) (`KismetMathLibrary.MakeRotator` _output_get) false false)
  (`self.NumberCheck`))

(fn `UserConstructionScript`)