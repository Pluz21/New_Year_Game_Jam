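; BP_BookTrigger1 is a trigger volume that calls RevealHidden when anything begins overlapping its Box.
; It binds OnReveal at BeginPlay to switch the debug color, and binds an empty OnConditionToRevealIsMet handler on each overlap before requesting the reveal.
; Tick draws the box bounds as a long-lived debug box every frame, so drawings accumulate.
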(event `self.ReceiveBeginPlay`
  (add `RevealHiddenComponent.onReveal` (`self.RevealHidden`) (delegate `onReveal_Event`)))

(event `onReveal_Event`
  (set `self.DebugColor` (`self.OnRevealColor`)))

(event `self.ReceiveTick`
  (params (DeltaSeconds :type "Float (single-precision)"))
  (bind _box (`self.Box`))
  (`KismetSystemLibrary.DrawDebugBox` (`SceneComponent.K2_GetComponentLocation` _box) (`BoxComponent.GetScaledBoxExtent` _box) (`self.DebugColor`) (struct) 100.0 2.0))

(event `self.Box.OnComponentBeginOverlap`
  (params (OverlappedComponent :type "PrimitiveComponent Object Reference") (OtherActor :type "Actor Object Reference") (OtherComp :type "PrimitiveComponent Object Reference") (OtherBodyIndex :type Integer) (bFromSweep :type Boolean) (SweepResult :type "HitResult Structure (by ref)"))
  (bind _revealhidden (`self.RevealHidden`))
  (add `RevealHiddenComponent.onConditionToRevealIsMet` _revealhidden (delegate `onConditionToRevealIsMet_Event`))
  (`RevealHiddenComponent.RevealHidden` _revealhidden))

(event `onConditionToRevealIsMet_Event`)

(fn `UserConstructionScript`)