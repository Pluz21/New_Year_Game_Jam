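; Three-tumbler combination lock that unlocks a linked BPUnlockable when its digits match Combination.
; Tick, throttled by a Delay, joins each child tumbler's TumblerNumber / 36 into a string for comparison, printing debug output.
; A match runs a one-time timed sequence: clears LockedState, briefly simulates lock physics and calls Unlock twice.
; A trigger box, sized and placed in construction, toggles the player's IsUsingLock on overlap.
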(event `self.ReceiveTick`
  (params (DeltaSeconds :type "Float (single-precision)"))
  ;[1 1 1] CorrectCombo Checker
  (`KismetSystemLibrary.Delay` 0.6)
  (bind _combomatches (`self.Check Combination`))
  (if _combomatches
    (`/Engine/EditorBlueprintResources/StandardMacros.DoOnce` false
      (:`Completed`
        (set `self.lockedState` false)
        (`KismetSystemLibrary.Delay` 1.4)
        (`SkeletalMeshComponent.SetAllBodiesSimulatePhysics` (`self.LockMesh`) true)
        (`KismetSystemLibrary.Delay` 0.4)
        (`/Game/GameJamContent/BP/LockCombo/BP_UnlockableParent.Unlock` (`self.BP_Unlockable`))
        (`KismetSystemLibrary.Delay` 0.2)
        (`SkeletalMeshComponent.SetAllBodiesSimulatePhysics` (`self.LockMesh`) false)
        (`KismetSystemLibrary.PrintString` "UNLOCK CALLED")
        (`/Game/GameJamContent/BP/LockCombo/BP_UnlockableParent.Unlock` (`self.BP_Unlockable`))))))

(event `self.ReceiveBeginPlay`)

(event `self.LockTriggerBox.OnComponentBeginOverlap`
  (params (OverlappedComponent :type "PrimitiveComponent Object Reference") (OtherActor :type "Actor Object Reference") (OtherComp :type "PrimitiveComponent Object Reference") (OtherBodyIndex :type Integer) (bFromSweep :type Boolean) (SweepResult :type "HitResult Structure (by ref)"))
  (bind _asbp_player (cast `/Game/GameJamContent/BP/Player/BP_Player` OtherActor))
  (set `/Game/GameJamContent/BP/Player/BP_Player.isUsingLock` true _asbp_player))

(event `self.LockTriggerBox.OnComponentEndOverlap`
  (params (OverlappedComponent :type "PrimitiveComponent Object Reference") (OtherActor :type "Actor Object Reference") (OtherComp :type "PrimitiveComponent Object Reference") (OtherBodyIndex :type Integer))
  (bind _asbp_player (cast `/Game/GameJamContent/BP/Player/BP_Player` OtherActor))
  (set `/Game/GameJamContent/BP/Player/BP_Player.isUsingLock` false _asbp_player))

(fn `Check Combination`
  (returns (comboMatches :type Boolean))
  (bind _returnvalue (`KismetStringLibrary.Conv_IntToString` (/ (`/Game/GameJamContent/BP/LockCombo/BP_LockTumble.tumblerNumber` (cast `/Game/GameJamContent/BP/LockCombo/BP_LockTumble` (`ChildActorComponent.ChildActor` (`self.BP_LockTumbler`)) :!pure true)) 36)))
  (bind _returnvalue_2 (`KismetStringLibrary.Conv_IntToString` (/ (`/Game/GameJamContent/BP/LockCombo/BP_LockTumble.tumblerNumber` (cast `/Game/GameJamContent/BP/LockCombo/BP_LockTumble` (`ChildActorComponent.ChildActor` (`self.BP_LockTumbler1`)) :!pure true)) 36)))
  (bind _returnvalue_3 (`KismetStringLibrary.Conv_IntToString` (/ (`/Game/GameJamContent/BP/LockCombo/BP_LockTumble.tumblerNumber` (cast `/Game/GameJamContent/BP/LockCombo/BP_LockTumble` (`ChildActorComponent.ChildActor` (`self.BP_LockTumbler2`)) :!pure true)) 36)))
  (bind _returnvalue_4 (== (`self.combination`) (`KismetStringLibrary.Concat_StrStr` _returnvalue _returnvalue_2 _returnvalue_3)))
  (`KismetSystemLibrary.PrintString` _returnvalue)
  (`KismetSystemLibrary.PrintString` _returnvalue_2)
  (`KismetSystemLibrary.PrintString` _returnvalue_3)
  (`KismetSystemLibrary.PrintString` (`KismetStringLibrary.Conv_BoolToString` _returnvalue_4) _returnvalue_4)
  (return _returnvalue_4))

(fn `UserConstructionScript`
  (bind _locktriggerbox (`self.LockTriggerBox`))
  (`SceneComponent.SetRelativeScale3D` _locktriggerbox (`self.lockTriggerBoxScale`))
  (`SceneComponent.K2_SetRelativeLocation` _locktriggerbox (`self.lockTriggerBoxOffset`) false false))