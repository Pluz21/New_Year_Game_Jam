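; BP_UnlockableParent is a base Blueprint for objects, such as doors, that animate open when unlocked.
; Its Unlock event drives UnlockableMesh with a timeline, either rotating it in yaw by RotateAmount or sliding it along relative X by MoveAmount.
; CanRotate takes priority over CanMove, and debug messages print during animation or when neither flag is set.
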(event `Unlock`
  (if (`self.canRotate`)
    (bind (_direction _alpha) (`Timeline|Timeline`)
      (:`Update`
        (`SceneComponent.K2_SetRelativeRotation` (`self.UnlockableMesh`) (`KismetMathLibrary.MakeRotator` 0.0 0.0 (* _alpha (`self.rotateAmount`))) false false)
        (`KismetSystemLibrary.PrintString` "Door unlock event called" true true (struct :`R` 1.0 :`B` 0.297794 :`A` 1.0))))
    (elif (`self.canMove`)
      (bind (_direction_2 _alpha_2) (`Timeline|Timeline_0`)
        (:`Update`
          (bind _returnvalue (* _alpha_2 (`self.moveAmount`)))
          (`SceneComponent.K2_SetRelativeLocation` (`self.UnlockableMesh`) (`KismetMathLibrary.MakeVector` _returnvalue) false false)
          (`KismetSystemLibrary.PrintString` (`KismetStringLibrary.Conv_DoubleToString` _returnvalue))))
      (else
        (`KismetSystemLibrary.PrintString` "Please use TRUE for move or rotate after unlock")))))

(fn `UserConstructionScript`)