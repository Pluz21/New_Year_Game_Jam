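; Three-tumbler combination lock that opens a linked unlockable when the player dials the correct code.
; Overlapping the trigger box, sized and placed by the construction script, toggles the player's IsUsingLock flag.
; A delayed Tick poll converts each child tumbler's TumblerNumber into a digit and compares the joined string to Combination.
; A match fires once, clearing LockedState, briefly simulating physics on the lock mesh and calling Unlock twice.
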(event `self.ReceiveTick`
  (params (DeltaSeconds :type "Float (single-precision)"))
  ;[1 1 1] CorrectCombo Checker
  (`KismetSystemLibrary.Delay` 0.6)
  (bind _combomatches (`self.Check Combination`))
  (if _combomatches
    (`/Engine/EditorBlueprintResources/StandardMacros.DoOnce` false
      (:`Completed`
        (set `self.lockedState` false)
        (`KismetSystemLibrary.Delay` 1.4)
        (`SkeletalMeshComponent.SetAllBodiesSimulatePhysics` (`self.LockMesh`) true)
        (`KismetSystemLibrary.Delay` 0.4)
        (`/Game/GameJamContent/BP/LockAssets/BP_Unlockable_With_Rotation_Designers.Unlock` (`self.BP_Unlockable`))
        (`KismetSystemLibrary.Delay` 0.2)
        (`SkeletalMeshComponent.SetAllBodiesSimulatePhysics` (`self.LockMesh`) false)
        (`/Game/GameJamContent/BP/LockAssets/BP_Unlockable_With_Rotation_Designers.Unlock` (`self.BP_Unlockable`))))))

(event `self.ReceiveBeginPlay`)

(event `self.LockTriggerBox.OnComponentBeginOverlap`
  (params (OverlappedComponent :type "PrimitiveComponent Object Reference") (OtherActor :type "Actor Object Reference") (OtherComp :type "PrimitiveComponent Object Reference") (OtherBodyIndex :type Integer) (bFromSweep :type Boolean) (SweepResult :type "HitResult Structure (by ref)"))
  (bind _asbp_player (cast `/Game/GameJamContent/BP/Player/BP_Player` OtherActor))
  (set `/Game/GameJamContent/BP/Player/BP_Player.isUsingLock` true _asbp_player))

(event `self.LockTriggerBox.OnComponentEndOverlap`
  (params (OverlappedComponent :type "PrimitiveComponent Object Reference") (OtherActor :type "Actor Object Reference") (OtherComp :type "PrimitiveComponent Object Reference") (OtherBodyIndex :type Integer))
  (bind _asbp_player (cast `/Game/GameJamContent/BP/Player/BP_Player` OtherActor))
  (set `/Game/GameJamContent/BP/Player/BP_Player.isUsingLock` false _asbp_player))

(fn `Check Combination`
  (returns (comboMatches :type Boolean))
  (return (== (`self.combination`) (`KismetStringLibrary.Concat_StrStr` (`KismetStringLibrary.Conv_IntToString` (/ (`/Game/GameJamContent/BP/LockAssets/BP_LockTumbler_Designers.tumblerNumber` (cast `/Game/GameJamContent/BP/LockAssets/BP_LockTumbler_Designers` (`ChildActorComponent.ChildActor` (`self.BP_LockTumbler`)) :!pure true)) 36)) (`KismetStringLibrary.Conv_IntToString` (/ (`/Game/GameJamContent/BP/LockAssets/BP_LockTumbler_Designers.tumblerNumber` (cast `/Game/GameJamContent/BP/LockAssets/BP_LockTumbler_Designers` (`ChildActorComponent.ChildActor` (`self.BP_LockTumbler1`)) :!pure true)) 36)) (`KismetStringLibrary.Conv_IntToString` (/ (`/Game/GameJamContent/BP/LockAssets/BP_LockTumbler_Designers.tumblerNumber` (cast `/Game/GameJamContent/BP/LockAssets/BP_LockTumbler_Designers` (`ChildActorComponent.ChildActor` (`self.BP_LockTumbler2`)) :!pure true)) 36))))))

(fn `UserConstructionScript`
  (bind _locktriggerbox (`self.LockTriggerBox`))
  (`SceneComponent.SetRelativeScale3D` _locktriggerbox (`self.lockTriggerBoxScale`))
  (`SceneComponent.K2_SetRelativeLocation` _locktriggerbox (`self.lockTriggerBoxOffset`) false false))