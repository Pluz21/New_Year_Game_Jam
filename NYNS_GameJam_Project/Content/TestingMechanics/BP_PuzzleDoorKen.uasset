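; BP_PuzzleDoorKen is a puzzle door that swings open once enough keys have been collected.
; CollectPuzzleDoorKey increments a counter, and when it reaches the required maximum a DoOnce waits one second and fires OpenPuzzleDoor.
; OpenPuzzleDoor plays a timeline that lerps the Door component's relative yaw to swing it open.
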(event `Open Puzzle Door`
  (bind (_direction _alpha) (`Timeline|Open Puzzle Door Animation`)
    (:`Update`
      (`SceneComponent.K2_SetRelativeRotation` (`self.Door`) (`KismetMathLibrary.MakeRotator` 0.0 0.0 (`KismetMathLibrary.Lerp` 0.0 -120.0 _alpha)) false false))))

(event `Collect PuzzleDoor Key`
  (`/Engine/EditorBlueprintResources/StandardMacros.IncrementInt` (`self.currentPuzzleKeyCollected`)
    (:`  `
      (if (>= (`self.currentPuzzleKeyCollected`) (`self.maxPuzzleKeyCollectables`))
        (`/Engine/EditorBlueprintResources/StandardMacros.DoOnce` false
          (:`Completed`
            (`KismetSystemLibrary.Delay` 1.0)
            (`self.Open Puzzle Door`)))))))

(fn `UserConstructionScript`)