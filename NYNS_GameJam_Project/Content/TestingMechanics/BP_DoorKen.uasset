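; BP_DoorKen is a swinging door that BP_Player can open and close, opening in a direction set by which side is approached.
; Two trigger boxes set opposite 90-degree yaw targets and tell the player whether it can open this door.
; OpenDoor caches the target, then plays or reverses a timeline that lerps absolute world rotation from zero.
; A moving flag ignores new requests until the timeline finishes.
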(event `self.Box01.OnComponentBeginOverlap`
  (params (OverlappedComponent :type "PrimitiveComponent Object Reference") (OtherActor :type "Actor Object Reference") (OtherComp :type "PrimitiveComponent Object Reference") (OtherBodyIndex :type Integer) (bFromSweep :type Boolean) (SweepResult :type "HitResult Structure (by ref)"))
  (set `self.DoorOpeningRotation` (struct :`Yaw` -90.0))
  (bind _asbp_player (cast `/Game/GameJamContent/BP/Player/BP_Player` OtherActor))
  (`/Game/GameJamContent/BP/Player/BP_Player.CanOpenDoor` _asbp_player true self))

(event `self.Box01.OnComponentEndOverlap`
  (params (OverlappedComponent :type "PrimitiveComponent Object Reference") (OtherActor :type "Actor Object Reference") (OtherComp :type "PrimitiveComponent Object Reference") (OtherBodyIndex :type Integer))
  (bind _asbp_player (cast `/Game/GameJamContent/BP/Player/BP_Player` OtherActor))
  (`/Game/GameJamContent/BP/Player/BP_Player.CanOpenDoor` _asbp_player false null))

(event `self.Box02.OnComponentBeginOverlap`
  (params (OverlappedComponent :type "PrimitiveComponent Object Reference") (OtherActor :type "Actor Object Reference") (OtherComp :type "PrimitiveComponent Object Reference") (OtherBodyIndex :type Integer) (bFromSweep :type Boolean) (SweepResult :type "HitResult Structure (by ref)"))
  (set `self.DoorOpeningRotation` (struct :`Yaw` 90.0))
  (bind _asbp_player (cast `/Game/GameJamContent/BP/Player/BP_Player` OtherActor))
  (`/Game/GameJamContent/BP/Player/BP_Player.CanOpenDoor` _asbp_player true self))

(event `self.Box02.OnComponentEndOverlap`
  (params (OverlappedComponent :type "PrimitiveComponent Object Reference") (OtherActor :type "Actor Object Reference") (OtherComp :type "PrimitiveComponent Object Reference") (OtherBodyIndex :type Integer))
  (bind _asbp_player (cast `/Game/GameJamContent/BP/Player/BP_Player` OtherActor))
  (`/Game/GameJamContent/BP/Player/BP_Player.CanOpenDoor` _asbp_player false null))

(event `OpenDoor`
  (params (OpenDoor :type Boolean))
  (if (not (`self.DoorIsCurrentlyMoving`))
    (set `self.DoorIsCurrentlyMoving` true)
    (bind _output_get (set `self.Open Door` OpenDoor))
    (if _output_get
      (set `self.Door Opening Rotation Temp` (`self.DoorOpeningRotation`))
      (bind (_direction _alpha) (`Timeline|DoorOpenAnimation` :!via `PlayFromStart` :!label _label)
        (:`Update`
          (`SceneComponent.K2_SetWorldRotation` (`self.Door`) (`KismetMathLibrary.RLerp` (struct) (`self.Door Opening Rotation Temp`) _alpha) false false))
        (:`Finished`
          (set `self.DoorIsCurrentlyMoving` false)))
      (else
        (goto _label :!via `Reverse`)))))

(fn `UserConstructionScript`)